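; Actor component that fades the materials of its owning Static Mesh Actor between full and partial fade levels.
; BeginPlay wraps each material slot in a dynamic material instance and does nothing further for other owner types.
; FadeIn and FadeOut set the target and enable Tick, which interpolates the FadeAmount scalar parameter across those instances.
; Tick stays off while idle, switching itself off once the value nears the target.
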(event `self.ReceiveBeginPlay`
  (`self.SetComponentTickEnabled` false)
  (bind _asstatic_mesh_actor (cast `StaticMeshActor` (`self.GetOwner`)))
  (bind _output_get (set `self.OwnerMesh` (`StaticMeshActor.StaticMeshComponent` _asstatic_mesh_actor)))
  (for _index (range (+ (`PrimitiveComponent.GetNumMaterials` _output_get) 1))
    (bind _returnvalue (`PrimitiveComponent.CreateDynamicMaterialInstance` (`self.OwnerMesh`) _index (`PrimitiveComponent.GetMaterial` _output_get _index) "None"))
    (`KismetArrayLibrary.Array_Add` (`self.DynamicMaterials`) _returnvalue)))

(event `self.ReceiveTick`
  (params (DeltaSeconds :type "Float (single-precision)"))
  (if (`KismetArrayLibrary.Array_IsNotEmpty` (`self.DynamicMaterials`))
    (set `self.CurrentFadeAmount` (`KismetMathLibrary.FInterpTo` (`self.CurrentFadeAmount`) (`self.TargetFadeAmount`) DeltaSeconds (`self.FadeSpeed`)))
    (for _array_element (`self.DynamicMaterials`)
      (`/Engine/EditorBlueprintResources/StandardMacros.IsValid` _array_element
        (:`Is Valid`
          (`MaterialInstanceDynamic.SetScalarParameterValue` _array_element "FadeAmount" (`self.CurrentFadeAmount`))
          (if (`KismetMathLibrary.NearlyEqual_FloatFloat` (`self.CurrentFadeAmount`) (`self.TargetFadeAmount`) 0.01)
            (set `self.CurrentFadeAmount` (`self.TargetFadeAmount`))
            (`self.SetComponentTickEnabled` false)))))))

(fn `FadeIn`
  (set `self.TargetFadeAmount` 1.0)
  (`self.SetComponentTickEnabled` true))

(fn `FadeOut`
  (set `self.TargetFadeAmount` 0.25)
  (`self.SetComponentTickEnabled` true))