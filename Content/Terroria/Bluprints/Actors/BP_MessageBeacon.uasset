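; BP_MessageBeacon is a box trigger actor that detects when the player character enters a named region.
; On begin overlap it compares its RegionName tag with the player's CurrentRegionName; if they differ, it debug-prints the old name, calls OnBeginOverlap, then stores the new name on the player.
; End overlap forwards any actor to OnEndOverlap unfiltered; neither handler is defined in this graph.
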(event `self.Box.OnComponentBeginOverlap`
  (params (OverlappedComponent :type "PrimitiveComponent Object Reference") (OtherActor :type "Actor Object Reference") (OtherComp :type "PrimitiveComponent Object Reference") (OtherBodyIndex :type Integer) (bFromSweep :type Boolean) (SweepResult :type "HitResult Structure (by ref)"))
  (bind _returnvalue (`BlueprintGameplayTagLibrary.GetTagName` (`self.RegionName`)))
  (bind _asbp_player_character (cast `/Game/Terroria/Bluprints/Player/BP_PlayerCharacter` OtherActor))
  (bind _currentregionname (`/Game/Terroria/Bluprints/Player/BP_PlayerCharacter.CurrentRegionName` _asbp_player_character))
  (if (!= _currentregionname _returnvalue)
    (`KismetSystemLibrary.PrintString` (`KismetStringLibrary.Conv_NameToString` _currentregionname))
    (`self.OnBeginOverlap` _asbp_player_character)
    (set `/Game/Terroria/Bluprints/Player/BP_PlayerCharacter.CurrentRegionName` _returnvalue _asbp_player_character)))

(event `self.Box.OnComponentEndOverlap`
  (params (OverlappedComponent :type "PrimitiveComponent Object Reference") (OtherActor :type "Actor Object Reference") (OtherComp :type "PrimitiveComponent Object Reference") (OtherBodyIndex :type Integer))
  (`self.OnEndOverlap` OtherActor))

(fn `UserConstructionScript`)