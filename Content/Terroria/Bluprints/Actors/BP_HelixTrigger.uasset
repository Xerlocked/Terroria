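; BP_HelixTrigger is a sphere trigger that toggles the GodMode gameplay tag on a linked PlaceActor based on player presence.
; On BeginPlay it moves a valid PlaceActor to its own X and Y, keeping that actor's Z, and adds the replicated tag.
; A BP_PlayerCharacter entering the sphere removes the tag and sets the mesh material to MI_Moon.
; Leaving restores the tag and switches the material to MI_Moonblood.
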(event `self.ReceiveBeginPlay`
  (bind (_returnvalue_x _returnvalue_y) (`KismetMathLibrary.BreakVector` (`self.K2_GetActorLocation`)))
  (bind (_returnvalue_x_2 _returnvalue_y_2 _returnvalue_z) (`KismetMathLibrary.BreakVector` (`self.K2_GetActorLocation` (`self.PlaceActor`))))
  (bind _placeactor (`self.PlaceActor`)
    (:`then`
      (`self.K2_SetActorLocation` _placeactor (`KismetMathLibrary.MakeVector` _returnvalue_x _returnvalue_y _returnvalue_z) false true)
      (`AbilitySystemBlueprintLibrary.AddLooseGameplayTags` (`self.PlaceActor`) (`BlueprintGameplayTagLibrary.MakeGameplayTagContainerFromTag` (struct :`TagName` "GodMode")) true))
    (:`else`)))

(event `self.Sphere.OnComponentBeginOverlap`
  (params (OverlappedComponent :type "PrimitiveComponent Object Reference") (OtherActor :type "Actor Object Reference") (OtherComp :type "PrimitiveComponent Object Reference") (OtherBodyIndex :type Integer) (bFromSweep :type Boolean) (SweepResult :type "HitResult Structure (by ref)"))
  (cast `/Game/Terroria/Bluprints/Player/BP_PlayerCharacter` OtherActor)
  (`PrimitiveComponent.SetMaterial` (`self.StaticMesh`) 0 "/Game/Necropolis/Materials/MI_Moon.MI_Moon")
  (`AbilitySystemBlueprintLibrary.RemoveLooseGameplayTags` (`self.PlaceActor`) (`BlueprintGameplayTagLibrary.MakeGameplayTagContainerFromTag` (struct :`TagName` "GodMode")) true))

(event `self.Sphere.OnComponentEndOverlap`
  (params (OverlappedComponent :type "PrimitiveComponent Object Reference") (OtherActor :type "Actor Object Reference") (OtherComp :type "PrimitiveComponent Object Reference") (OtherBodyIndex :type Integer))
  (cast `/Game/Terroria/Bluprints/Player/BP_PlayerCharacter` OtherActor)
  (`PrimitiveComponent.SetMaterial` (`self.StaticMesh`) 0 "/Game/Necropolis/Materials/MI_Moonblood.MI_Moonblood")
  (`AbilitySystemBlueprintLibrary.AddLooseGameplayTags` (`self.PlaceActor`) (`BlueprintGameplayTagLibrary.MakeGameplayTagContainerFromTag` (struct :`TagName` "GodMode")) true))

(fn `UserConstructionScript`)