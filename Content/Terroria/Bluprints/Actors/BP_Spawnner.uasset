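; Server-authoritative spawner that keeps a capped population of a configurable actor class inside a sphere boundary.
; On BeginPlay it runs a spawn pass and starts a looping timer to refill on an interval.
; Each pass fills the container up to the max count at random navigable points with random yaw.
; Destroyed actors leave the container through a bound OnDestroyed event, freeing slots for later spawns.
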(event `self.ReceiveBeginPlay`
  (`/Engine/EditorBlueprintResources/ActorMacros.Switch Has Authority`
    (:`Authority`
      (`self.SpawnActorEvent`)
      (bind _returnvalue (`KismetSystemLibrary.K2_SetTimerDelegate` (`|CreateDelegate` :!event `SpawnActorEvent`) (`self.SpawnTime`) true))
      (set `self.SpawnTimerHandle` _returnvalue))))

(event `SpawnActorEvent`
  (bind _sphere_boundary (`self.Sphere Boundary`))
  (for _ (range (+ (`self.MaxSpawnCount`) 1))
    (if (< (`KismetArrayLibrary.Array_Length` (`self.SpawnContainer`)) (`self.MaxSpawnCount`))
      (bind _randomlocation (`NavigationSystemV1.K2_GetRandomLocationInNavigableRadius` (`NavigationSystemV1.GetNavigationSystem`) (`SceneComponent.K2_GetComponentLocation` _sphere_boundary) (`SphereComponent.SphereRadius` _sphere_boundary) null null))
      (bind _returnvalue (`|SpawnActorFromClass` (`self.SpawnActorFromClass`) (`KismetMathLibrary.MakeTransform` _randomlocation (`KismetMathLibrary.MakeRotator` 0.0 0.0 (.yaw (`KismetMathLibrary.RandomRotator` false)))) "AdjustIfPossibleButAlwaysSpawn" "MultiplyWithRoot" null null))
      (`KismetArrayLibrary.Array_AddUnique` (`self.SpawnContainer`) _returnvalue)
      (add `self.OnDestroyed` _returnvalue (delegate `OnDestroyActor`)))))

(event `OnDestroyActor` :!signature `self.OnDestroyed`
  (params (DestroyedActor :type "Actor Object Reference"))
  (`KismetArrayLibrary.Array_RemoveItem` (`self.SpawnContainer`) DestroyedActor))

(fn `UserConstructionScript`)