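; Gold pickup drop that shows its amount on a floating WBP_GoldOverlay label and refreshes it when the amount updates.
; The label hides during cinematic camera mode through the player controller's camera-mode event.
; On sphere overlap with the player, it adds the amount to BP_TPlayerState gold, destroys itself and unbinds that event.
; An extra hard-coded million-gold grant, commented "Delete", also runs on every pickup.
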(event `OnCameraModeChange_Event`
  (params (bIsCinematic :type Boolean))
  (bind _labelwidgetcomponent (`self.LabelWidgetComponent`))
  (if bIsCinematic
    (`SceneComponent.SetVisibility` _labelwidgetcomponent false false)
    (else
      (`SceneComponent.SetVisibility` _labelwidgetcomponent true false))))

(event `self.ReceiveBeginPlay`
  (bind _aswbp_gold_overlay (cast `/Game/Terroria/UI/Item/WBP_GoldOverlay` (`WidgetComponent.GetWidget` (`self.LabelWidgetComponent`))))
  (`/Game/Terroria/UI/Item/WBP_GoldOverlay.SetGoldText` _aswbp_gold_overlay (`self.ItemAmount`))
  (bind _asbp_player_controller (cast `/Game/Terroria/Bluprints/Controller/BP_PlayerController` (`GameplayStatics.GetPlayerController` 0)))
  (add `TPlayerController.OnCameraModeChange` _asbp_player_controller (`|CreateDelegate` :!event `OnCameraModeChange_Event`)))

(event `self.Sphere.OnComponentBeginOverlap`
  (params (OverlappedComponent :type "PrimitiveComponent Object Reference") (OtherActor :type "Actor Object Reference") (OtherComp :type "PrimitiveComponent Object Reference") (OtherBodyIndex :type Integer) (bFromSweep :type Boolean) (SweepResult :type "HitResult Structure (by ref)"))
  (if (`self.ActorHasTag` OtherActor "Player")
    (bind _asbp_player_character (cast `/Game/Terroria/Bluprints/Player/BP_PlayerCharacter` OtherActor))
    (bind _asbp_tplayer_state (cast `/Game/Terroria/Bluprints/Player/BP_TPlayerState` (`Pawn.PlayerState` _asbp_player_character)))
    (`TPlayerState.AddToGold` _asbp_tplayer_state (`self.ItemAmount`))
    ;[0.01161 0.01161 0.01161] Delete
    (`TPlayerState.AddToGold` _asbp_tplayer_state 1000000)
    (`self.K2_DestroyActor`)
    (bind _asbp_player_controller (cast `/Game/Terroria/Bluprints/Controller/BP_PlayerController` (`GameplayStatics.GetPlayerController` 0)))
    (remove `TPlayerController.OnCameraModeChange` _asbp_player_controller (`|CreateDelegate` :!event `OnCameraModeChange_Event`))))

(event `self.ReceiveItemAmountUpdated`
  (params (Amount :type Integer))
  (bind _aswbp_gold_overlay (cast `/Game/Terroria/UI/Item/WBP_GoldOverlay` (`WidgetComponent.GetWidget` (`self.LabelWidgetComponent`))))
  (`/Game/Terroria/UI/Item/WBP_GoldOverlay.SetGoldText` _aswbp_gold_overlay Amount))

(fn `UserConstructionScript`)