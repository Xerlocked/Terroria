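; AI controller for the Helix boss that drives its behavior tree and player detection.
; On possession it stores the Helix boss reference and runs BT_Helix.
; When perception senses an actor tagged Player, it writes that actor to the blackboard target key and calls CallOnTargeting on the boss.
; Losing sight of the target is not handled, so the blackboard target is never cleared here.
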(event `self.ReceivePossess`
  (params (PossessedPawn :type "Pawn Object Reference"))
  (bind _asbp_boss_helix (cast `/Game/Terroria/Bluprints/Enemy/BP_Boss_Helix` PossessedPawn))
  (set `self.BP Boss Helix` _asbp_boss_helix)
  (`self.RunBehaviorTree` "/Game/Terroria/AI/BT_Helix.BT_Helix"))

(event `self.PerceptionComponent.OnTargetPerceptionUpdated`
  (params (Actor :type "Actor Object Reference") (Stimulus :type "AIStimulus Structure"))
  (if (and (`self.ActorHasTag` Actor "Player") (`.bSuccessfullySensed` (break `AIStimulus` Stimulus)))
    (`BlackboardComponent.SetValueAsObject` (`AIBlueprintHelperLibrary.GetBlackboard` null) (`self.TargetActorKey`) Actor)
    (`/Game/Terroria/Bluprints/Enemy/BP_Boss_Helix.OnTargeting` (`self.BP Boss Helix`) Actor)))

(fn `UserConstructionScript`)