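; GA_DarkShield is the Warlock's Dark Shield gameplay ability, which applies a shield effect to the caster during a power-up montage.
; On activation it commits, applies an ignore-movement-input effect, and plays the montage.
; The montage's DarkShield gameplay event triggers GE_Shield on the avatar's ability system component, followed by ApplyActiveEffect.
; Any montage exit ends the ability, and ending it removes the movement lock through its stored handle.
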(event `self.K2_ActivateAbility`
  (bind _returnvalue (`AbilitySystemBlueprintLibrary.GetAbilitySystemComponent` (`self.GetAvatarActorFromActorInfo`)))
  (`self.K2_CommitAbility`)
  (bind _returnvalue_2 (`self.BP_ApplyGameplayEffectToOwner` "/Game/Terroria/AbilitySystem/GameplayEffects/Player/GE_IgnoreMovementInput.GE_IgnoreMovementInput_C"))
  (set `self.IgnoreHandle` _returnvalue_2)
  (`AbilityTask_PlayMontageAndWait.CreatePlayMontageAndWaitProxy` "None" "/Game/Terroria/Animations/Warlock/Animation_Shield_Powerup_Montage.Animation_Shield_Powerup_Montage"
    (:`then`
      (`AbilityTask_WaitGameplayEvent.WaitGameplayEvent` (struct :`TagName` "Event.Montage.DarkShield") null
        (:`EventReceived`
          (`AbilitySystemComponent.BP_ApplyGameplayEffectToSelf` _returnvalue "/Game/Terroria/AbilitySystem/GameplayEffects/Player/GE_Shield.GE_Shield_C" 0.0 (`AbilitySystemComponent.MakeEffectContext` _returnvalue))
          (`self.ApplyActiveEffect` _returnvalue))))
    (:`OnCompleted`
      (`self.K2_EndAbility` :!label _label))
    (:`OnBlendOut`
      (goto _label))
    (:`OnInterrupted`
      (goto _label))
    (:`OnCancelled`
      (goto _label))))

(event `self.K2_OnEndAbility`
  (params (bWasCancelled :type Boolean))
  (`AbilitySystemComponent.RemoveActiveGameplayEffect` (`AbilitySystemBlueprintLibrary.GetAbilitySystemComponent` (`self.GetAvatarActorFromActorInfo`)) (`self.IgnoreHandle`) -1))