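; Actor for the Warlock's Black Hole ability that applies a gameplay effect to nearby pawns once, on BeginPlay.
; A sphere overlap of ScanRadius around the actor gathers pawns, excluding the instigator.
; The instigator's Ability System Component applies EffectSpecHandle to each pawn that has its own ASC.
; A debug sphere shows the scan area; the graph has no ticking or pull logic.
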(event `self.ReceiveBeginPlay`
  (bind _returnvalue (`self.K2_GetActorLocation`))
  (bind _returnvalue_2 (`self.GetInstigator`))
  (bind _scanradius (`self.ScanRadius`))
  (bind _returnvalue_3 (`AbilitySystemBlueprintLibrary.GetAbilitySystemComponent` _returnvalue_2))
  (`KismetSystemLibrary.DrawDebugSphere` _returnvalue _scanradius 12 (struct :`R` 1.0 :`G` 0.603158 :`B` 0.6 :`A` 1.0) 10.0 2.0)
  (bind _outactors (`KismetSystemLibrary.SphereOverlapActors` _returnvalue _scanradius (`|MakeArray` "ObjectTypeQuery3" :!type "EObjectTypeQuery Enum") null (`|MakeArray` _returnvalue_2 :!type "Actor Object Reference")))
  (for _array_element _outactors
    (bind _returnvalue_4 (`AbilitySystemBlueprintLibrary.GetAbilitySystemComponent` _array_element))
    (`/Engine/EditorBlueprintResources/StandardMacros.IsValid` _returnvalue_4
      (:`Is Valid`
        (`/Engine/EditorBlueprintResources/StandardMacros.IsValid` _returnvalue_3
          (:`Is Valid`
            (`AbilitySystemComponent.BP_ApplyGameplayEffectSpecToTarget` _returnvalue_3 (`self.EffectSpecHandle`) _returnvalue_4)))))))

(fn `UserConstructionScript`)