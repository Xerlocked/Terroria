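; GA_BlackHole is a Warlock gameplay ability that places a black hole at a targeted location.
; On activation it waits for user-confirmed target data, showing a black hole reticle.
; A blocking hit commits the ability and spawns BP_BlackHole there with a scan radius and a damage effect spec built via a SetByCaller magnitude.
; It ends on valid data or cancellation, printing a debug message when nothing blocks.
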(event `self.K2_ActivateAbility`
  (bind _returnvalue (`self.GetAbilitySystemComponentFromActorInfo`))
  (bind (_asynctaskproxy _data) (`AbilityTask_WaitTargetData.WaitTargetData` "None" "UserConfirmed" "/Script/Terroria.TGameplayAbilityTargetActor" 1500.0 (struct) (struct) "/Game/Terroria/AbilitySystem/GameplayAbilities/Warlock/4_BlackHole/GARet_BlackHole.GARet_BlackHole_C")
    (:`then`
      (`KismetSystemLibrary.PrintString` "BlackHole Active"))
    (:`ValidData`
      (bind (_bblockinghit _binitialoverlap _time _distance _location) (`GameplayStatics.BreakHitResult` (`AbilitySystemBlueprintLibrary.GetHitResultFromTargetData` _data)))
      (if _bblockinghit
        (`self.K2_CommitAbility`)
        (bind _returnvalue_2 (`AbilitySystemBlueprintLibrary.AssignTagSetByCallerMagnitude` (`AbilitySystemComponent.MakeOutgoingSpec` _returnvalue "/Game/Terroria/AbilitySystem/GameplayEffects/GE_DamageSample.GE_DamageSample_C" 1.0 (`AbilitySystemComponent.MakeEffectContext` _returnvalue)) (struct :`TagName` "Damage") 80.0))
        (`|SpawnActorFromClass` "/Game/Terroria/AbilitySystem/GameplayAbilities/Warlock/4_BlackHole/BP_BlackHole.BP_BlackHole_C" (`KismetMathLibrary.MakeTransform` _location) "AlwaysSpawn" "MultiplyWithRoot" null 300.0 _returnvalue_2 (`Actor.Instigator` (`self.GetOwningActorFromActorInfo`)))
        (else
          (`KismetSystemLibrary.PrintString` "Not Blocking : BlackHole")))
      (`self.K2_EndAbility`))
    (:`Cancelled`
      (`self.K2_EndAbility`))))